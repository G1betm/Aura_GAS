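; BP_FlamePillar is a flame pillar actor whose point light flickers by varying its intensity over time.
; From BeginPlay, it randomly plays one of two intensity timelines and picks again whenever one finishes, giving a continuous, varied loop.
; Each timeline update passes its curve value to ScaleFlameIntensity, which multiplies it by BaseIntensity and applies it to the PointLight.
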(event Custom|StartTimelime_1
  (bind _flameintensity (Timeline|FlameIntensity1 PlayFromStart)
    (:Update
      (CallFunction|ScaleFlameIntensity _flameintensity))
    (:Finished
      (CallFunction|ChooseTimeline))))

(event Custom|StartTimelime_2
  (bind _flameintensity (Timeline|FlameIntensity2 PlayFromStart)
    (:Update
      (CallFunction|ScaleFlameIntensity _flameintensity))
    (:Finished
      (CallFunction|ChooseTimeline))))

(event Custom|ChooseTimeline
  (switch int (Math|Random|RandomIntegerinRange 0 1)
    (:Default
      (CallFunction|StartTimelime2))
    (:0
      (CallFunction|StartTimelime1))
    (:1
      (CallFunction|StartTimelime2))))

(event EventBeginPlay
  (CallFunction|ChooseTimeline))

(fn ConstructionScript)

(fn ScaleFlameIntensity
  (params (Intensity :type Float%20%28double-precision%29))
  (Rendering|Components|Light|SetIntensity (Variables|Default|GetPointLight) (* Intensity (Variables|Default|GetBaseIntensity))))