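; GA_RangedAttack is an enemy gameplay ability that fires a projectile at the combat target.
; On activation it caches the target's location, updates the avatar's motion warp target and plays a random tagged attack montage.
; The montage's gameplay event spawns the projectile from the tagged socket toward that cached location, with an optional pitch override.
; The ability ends when the montage completes, is interrupted or is cancelled.
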(event Ability|EventActivateAbility
  (bind _returnvalue (Ability|GetAvatarActorfromActorInfo))
  (bind _returnvalue_2 (Class|EnemyInterface|GetCombatTarget(Message) _returnvalue))
  (bind _output_get (Variables|Default|SetCombatTargetLocation (Transformation|GetActorLocation _returnvalue_2)))
  (Class|CombatInterface|UpdateWarpTarget(Message) _returnvalue _output_get)
  (bind _returnvalue_3 (Class|CombatInterface|GetAttackMontages(Message) (Ability|GetAvatarActorfromActorInfo)))
  (bind _output_get_2 (Variables|Default|SetTaggedMontage (Class|AuraDamageGameplayAbility|GetRandomTaggedMontage _returnvalue_3)))
  (|PlayMontageandWaitProxy "None" (.Montage (Utilities|Struct|BreakTaggedMontage _output_get_2)) 1.0 "None" true 1.0 0.0 false
    (:then
      (Ability|Tasks|WaitGameplayEvent (.MontageTag (Utilities|Struct|BreakTaggedMontage _output_get_2)) 0 true
        (:EventReceived
          (Class|AuraProjectileSpell|SpawnProjectile (Variables|Default|GetCombatTargetLocation) (.SocketTag (Utilities|Struct|BreakTaggedMontage _output_get_2)) (Variables|Default|GetShouldOverridePitch) (Variables|Default|GetPithOverride)))))
    (:OnCompleted
      (Ability|EndAbility :!label _label))
    (:OnInterrupted
      (goto _label))
    (:OnCancelled
      (goto _label))))

(event Ability|EventOnEndAbility
  (params (bWasCancelled :type Boolean)))