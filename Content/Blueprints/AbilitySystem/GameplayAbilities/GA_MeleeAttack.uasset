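; GA_MeleeAttack is a gameplay ability for a melee attack that plays the goblin spear attack montage.
; On activation it sets the avatar's warp target to its combat target's location, then plays the montage.
; When the melee montage event arrives, it finds live players within a small radius of the combat socket and draws debug spheres on them, applying no damage.
; The ability ends when the montage completes, is interrupted or is cancelled.
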(event Ability|EventActivateAbility
  (bind _returnvalue (Ability|GetAvatarActorfromActorInfo))
  (bind _returnvalue_2 (Ability|GetAvatarActorfromActorInfo))
  (bind _returnvalue_3 (Class|EnemyInterface|GetCombatTarget(Message) _returnvalue_2))
  (bind _ascombat_interface (Utilities|Casting|CastToCombatInterface _returnvalue_2))
  (Class|CombatInterface|UpdateWarpTarget _ascombat_interface (Transformation|GetActorLocation _returnvalue_3))
  (|PlayMontageandWaitProxy "None" "/Game/Assets/Enemies/Goblin/Animations/Spear/AM_AttackGoblinSpear.AM_AttackGoblinSpear" 1.0 "None" true 1.0 0.0 false
    (:then
      (Ability|Tasks|WaitGameplayEvent "(TagName=\"Event.Montage.Attack.Melee\")" 0
        (:EventReceived
          (bind _returnvalue_4 (Class|CombatInterface|GetCombatSocketLocation(Message) _returnvalue))
          (bind _outoverlappingactors (Class|AuraAbilitySystemLibrary|GetLivePlayersWithinRadius _returnvalue (Utilities|Array|MakeArray _returnvalue) 45.0 _returnvalue_4))
          (for _array_element _outoverlappingactors
            (Rendering|Debug|DrawDebugSphere (Transformation|GetActorLocation _array_element) 15.0 12 "(R=1.000000,G=0.834380,B=0.000000,A=1.000000)" 1.0)))))
    (:OnCompleted
      (Ability|EndAbility :!label _label))
    (:OnInterrupted
      (goto _label))
    (:OnCancelled
      (goto _label))))

(event Ability|EventOnEndAbility
  (params (bWasCancelled :type Boolean)))