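; BP_Checkpoint is a checkpoint actor that gives visual feedback when it is reached or highlighted.
; CheckpointReached plays a timeline that drives the Glow parameter of the supplied dynamic material instance, scaled by GlowFactor.
; HighlightActor and UnHighlightActor toggle custom depth rendering on the checkpoint mesh, with highlighting also setting a stencil value.
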(event EventBeginPlay)

(event EventTick
  (params (DeltaSeconds :type Float%20%28single-precision%29)))

(event EventCheckpointReached
  (params (DynamicMaterialInstance :type Material%20Instance%20Dynamic%20Object%20Reference))
  (bind _glowtrack (Timeline|GlowTimeline Play)
    (:Update
      (Rendering|Material|SetScalarParameterValue DynamicMaterialInstance "Glow" (* _glowtrack (Variables|Default|GetGlowFactor)) :!class /Script/Engine.MaterialInstanceDynamic))))

(event EventHighlightActor
  (bind _checkpointmesh (Variables|Default|GetCheckpointMesh))
  (Rendering|SetRenderCustomDepth _checkpointmesh true)
  (Rendering|SetCustomDepthStencilValue _checkpointmesh 252))

(event EventUnHighlightActor
  (Rendering|SetRenderCustomDepth (Variables|Default|GetCheckpointMesh) false))

(fn ConstructionScript)